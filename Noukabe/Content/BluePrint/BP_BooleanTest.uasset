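; BP_BooleanTest is a test Blueprint that carves meshes out of a target mesh at runtime using boolean subtraction.
; BeginPlay gathers DynamicPMCActor instances tagged "OtherMesh" into OutActors and prints their count.
; The Subtract function subtracts each gathered actor from BooleanTargetMesh via BooleanWithMesh, destroys that actor, then prints a success message.
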(event `self.ReceiveBeginPlay`
  (bind _outactors (`GameplayStatics.GetAllActorsOfClassWithTag` "/Script/RuntimeGeometryUtils.DynamicPMCActor" "OtherMesh"))
  (bind _output_get (set `self.Out Actors` _outactors))
  (`KismetSystemLibrary.PrintString` (`KismetStringLibrary.Conv_IntToString` (`KismetArrayLibrary.Array_Length` _output_get))))

(event `self.ReceiveTick`
  (params (DeltaSeconds :type "Float (single-precision)")))

(fn `Subtract`
  (for _array_element (`self.Out Actors`)
    (`DynamicMeshBaseActor.BooleanWithMesh` (`self.BooleanTargetMesh`) _array_element "Subtraction")
    (`self.K2_DestroyActor` _array_element))
  (`KismetSystemLibrary.PrintString` "Success"))

(fn `UserConstructionScript`)