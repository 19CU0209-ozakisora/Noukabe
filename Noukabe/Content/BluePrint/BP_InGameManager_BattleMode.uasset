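; Battle-mode game manager that, after a start delay, spawns a set number of moving BP_Wall2PMask walls shaped from the 2P mocap player's pose.
; On each timed spawn it exports a render target to PNG, reloads it via DownloadImage as the wall's mask texture, and aligns hit spheres to six body sockets.
; DeleteWall counts removed walls and sets Clear; the effects-and-Result-level clear sequence exists but is never called.
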(event `self.ReceiveBeginPlay`
  ;[1 1 1] 壁生成位置設定
  (bind _output_get (set `self.WallGeneratePos` (`SceneComponent.K2_GetComponentLocation` (`self.WallGeneratePosActor`))))
  (`KismetSystemLibrary.PrintString` (`KismetStringLibrary.Concat_StrStr` "Wall Generate Pos : " (`KismetStringLibrary.Conv_VectorToString` _output_get)) true true (struct :`G` 1.0 :`A` 1.0) 5.0)
  ;[1 1 1] 壁削除位置設定
  (bind _output_get_2 (set `self.WallDeletePos` (`SceneComponent.K2_GetComponentLocation` (`self.WallDeletePosActor`))))
  (`KismetSystemLibrary.PrintString` (`KismetStringLibrary.Concat_StrStr` "Wall Delete Pos : " (`KismetStringLibrary.Conv_VectorToString` _output_get_2)) true true (struct :`G` 1.0 :`A` 1.0) 5.0)
  ;[1 1 1] 壁を流す長さ算出（現時点で算出結果は未使用）
  (bind _output_get_3 (set `self.WallFlowDistance` (`KismetMathLibrary.VSizeXY` (- (`self.WallGeneratePos`) (`self.WallDeletePos`)))))
  (`KismetSystemLibrary.PrintString` (`KismetStringLibrary.Concat_StrStr` "WallFlowDistance : " (`KismetStringLibrary.Conv_DoubleToString` _output_get_3)) true true (struct :`G` 1.0 :`A` 1.0) 5.0)
  ;[1 1 1] ゲーム状態設定
  (set `self.GameState` "NewEnumerator4")
  ;[1 1 1] 2P用モデル検索
  (bind _returnvalue (`GameplayStatics.GetActorOfClass` "/Game/BluePrint/MocapForAllTest.MocapForAllTest_C"))
  (bind _output_get_4 (set `self.Human` _returnvalue))
  (if (`KismetSystemLibrary.IsValid` _output_get_4)
    (`KismetSystemLibrary.PrintString` "Human is Valid" true true (struct :`G` 0.66 :`B` 1.0 :`A` 1.0) 3.0)
    (else
      (`KismetSystemLibrary.PrintString` "Human is NOT Valid!" true true (struct :`R` 1.0 :`A` 1.0) 10.0))))

(event `self.ReceiveTick`
  (params (DeltaSeconds :type "Float (single-precision)"))
  (set `self.DeltaTime` DeltaSeconds)
  (`|ExecutionSequence`
    (:`then_0`
      (switch `/Game/Other/InGameState` (`self.GameState`)
        (:`NewEnumerator4`
          (`KismetSystemLibrary.Delay` (`self.StartWallFlowTime`))
          (set `self.GameState` "NewEnumerator0")
          (`KismetSystemLibrary.PrintString` "GameStart!" true true (struct :`G` 1.0 :`A` 1.0) 3.0))
        (:`NewEnumerator0`
          (if (< (`self.GeneratedWallNum`) (`self.WallGenerateNumOneGame`))
            (bind _output_get (set `self.WallGenerateTimeCnt` (+ (`self.DeltaTime`) (`self.WallGenerateTimeCnt`))))
            (if (>= _output_get (`self.WallGenerateSpan`))
              (set `self.WallGenerateTimeCnt` 0.0)
              (`KismetSystemLibrary.PrintString` "Caputure" true true (struct :`G` 0.66 :`B` 1.0 :`A` 1.0) 5.0)
              (bind _output_get_2 (set `self.MaskTextureSavePath` (`KismetStringLibrary.Concat_StrStr` (`KismetSystemLibrary.GetProjectContentDirectory`) "/texture/SceneCapture/MaskTex")))
              (`ImageWriteBlueprintLibrary.ExportToDisk` "/Game/Other/NewTextureRenderTarget2D.NewTextureRenderTarget2D" _output_get_2 (make `ImageWriteOptions` "PNG" (delegate `CustomEvent`))))))))
    (:`then_1`
      (`KismetSystemLibrary.PrintString` (`KismetStringLibrary.Concat_StrStr` "GameState : " (`|GetEnumeratorNameAsString` (`self.GameState`))) true true (struct :`G` 1.0 :`A` 1.0) (`self.DeltaTime`)))))

(event `CustomEvent`
  (params (bSuccess :type Boolean))
  (bind _human (`self.Human`))
  (bind _generatedwall (`self.GeneratedWall`))
  (bind _generatedwall_2 (`self.GeneratedWall`))
  (bind _returnvalue (`self.K2_GetActorLocation` _generatedwall_2))
  (bind _skeletalmesh (`/Game/BluePrint/MocapForAllTest.SkeletalMesh` _human))
  (bind _spherecolforhead (`/Game/BluePrint/BP_Wall2PMask.SphereColForHead` _generatedwall_2))
  (bind _spherecolforlefthand (`/Game/BluePrint/BP_Wall2PMask.SphereColForLeftHand` _generatedwall_2))
  (bind _spherecolforleftleg (`/Game/BluePrint/BP_Wall2PMask.SphereColForLeftLeg` _generatedwall_2))
  (bind _spherecolforrighthand (`/Game/BluePrint/BP_Wall2PMask.SphereColForRightHand` _generatedwall_2))
  (bind _spherecolforrightleg (`/Game/BluePrint/BP_Wall2PMask.SphereColForRightLeg` _generatedwall_2))
  (bind _spherecolforspine (`/Game/BluePrint/BP_Wall2PMask.SphereColForSpine` _generatedwall_2))
  (bind _returnvalue_2 (- _returnvalue (`self.K2_GetActorLocation` _human)))
  (bind _y (.y _returnvalue))
  (bind (_returnvalue_x _returnvalue_y _returnvalue_z) (`KismetMathLibrary.BreakVector` (+ _returnvalue_2 (`SceneComponent.GetSocketLocation` _skeletalmesh "Socket_Head"))))
  (bind (_returnvalue_x_2 _returnvalue_y_2 _returnvalue_z_2) (`KismetMathLibrary.BreakVector` (+ _returnvalue_2 (`SceneComponent.GetSocketLocation` _skeletalmesh "Socket_L_Leg"))))
  (bind (_returnvalue_x_3 _returnvalue_y_3 _returnvalue_z_3) (`KismetMathLibrary.BreakVector` (+ _returnvalue_2 (`SceneComponent.GetSocketLocation` _skeletalmesh "Socket_Spine"))))
  (bind (_returnvalue_x_4 _returnvalue_y_4 _returnvalue_z_4) (`KismetMathLibrary.BreakVector` (+ _returnvalue_2 (`SceneComponent.GetSocketLocation` _skeletalmesh "Socket_R_Hand"))))
  (bind (_returnvalue_x_5 _returnvalue_y_5 _returnvalue_z_5) (`KismetMathLibrary.BreakVector` (+ _returnvalue_2 (`SceneComponent.GetSocketLocation` _skeletalmesh "Socket_L_Hand"))))
  (bind (_returnvalue_x_6 _returnvalue_y_6 _returnvalue_z_6) (`KismetMathLibrary.BreakVector` (+ _returnvalue_2 (`SceneComponent.GetSocketLocation` _skeletalmesh "Socket_R_Leg"))))
  (bind _texture (`AsyncTaskDownloadImage.DownloadImage` (`KismetStringLibrary.Concat_StrStr` "file:///" (`KismetSystemLibrary.GetProjectContentDirectory`) "/texture/SceneCapture/MaskTex.png"))
    (:`OnSuccess`
      (bind _returnvalue_3 (`|SpawnActorFromClass` "/Game/BluePrint/BP_Wall2PMask.BP_Wall2PMask_C" (`KismetMathLibrary.MakeTransform` (`self.WallGeneratePos`) (`self.WallRotation`) (`self.WallScale`)) "Undefined" "OverrideRootScale" null null))
      (bind _output_get (set `self.GeneratedWall` _returnvalue_3))
      (bind _wallmesh (`/Game/BluePrint/BP_Wall2PMask.WallMesh` _output_get))
      (bind _returnvalue_4 (`PrimitiveComponent.CreateDynamicMaterialInstance` _wallmesh 0 (`PrimitiveComponent.GetMaterial` _wallmesh 0) "None"))
      (`PrimitiveComponent.SetMaterial` _wallmesh 0 _returnvalue_4)
      (`MaterialInstanceDynamic.SetTextureParameterValue` _returnvalue_4 "MaskTexture" _texture)
      (set `/Game/BluePrint/BP_Wall2PMask.WallStartPos` (`self.WallGeneratePos`) _generatedwall)
      (set `/Game/BluePrint/BP_Wall2PMask.WallGoalPos` (`self.WallDeletePos`) _generatedwall)
      (set `/Game/BluePrint/BP_Wall2PMask.WallLifeTime` (`self.WallLifeTimeStartToGoal`) _generatedwall)
      (`SceneComponent.K2_SetWorldLocation` _spherecolforleftleg (`KismetMathLibrary.MakeVector` _returnvalue_x_2 _y (+ _returnvalue_z_2 (`self.ColZPosCorrectionValue`))) false false)
      (`SphereComponent.SetSphereRadius` _spherecolforleftleg (`self.SphereColRadius`) true)
      (`SceneComponent.K2_SetWorldLocation` _spherecolforrightleg (`KismetMathLibrary.MakeVector` _returnvalue_x_6 _y (+ _returnvalue_z_6 (`self.ColZPosCorrectionValue`))) false false)
      (`SphereComponent.SetSphereRadius` _spherecolforrightleg (`self.SphereColRadius`) true)
      (`SceneComponent.K2_SetWorldLocation` _spherecolforlefthand (`KismetMathLibrary.MakeVector` _returnvalue_x_5 _y (+ _returnvalue_z_5 (`self.ColZPosCorrectionValue`))) false false)
      (`SphereComponent.SetSphereRadius` _spherecolforlefthand (`self.SphereColRadius`) true)
      (`SceneComponent.K2_SetWorldLocation` _spherecolforrighthand (`KismetMathLibrary.MakeVector` _returnvalue_x_4 _y (+ _returnvalue_z_4 (`self.ColZPosCorrectionValue`))) false false)
      (`SphereComponent.SetSphereRadius` _spherecolforrighthand (`self.SphereColRadius`) true)
      (`SceneComponent.K2_SetWorldLocation` _spherecolforspine (`KismetMathLibrary.MakeVector` _returnvalue_x_3 _y (+ _returnvalue_z_3 (`self.ColZPosCorrectionValue`))) false false)
      (`SphereComponent.SetSphereRadius` _spherecolforspine (`self.SphereColRadius`) true)
      (`SceneComponent.K2_SetWorldLocation` _spherecolforhead (`KismetMathLibrary.MakeVector` _returnvalue_x _y (+ _returnvalue_z (`self.ColZPosCorrectionValue`))) false false)
      (`SphereComponent.SetSphereRadius` _spherecolforhead (`self.SphereColRadius`) true)
      (bind _output_get_2 (set `self.GeneratedWallNum` (+ (`self.GeneratedWallNum`) 1)))
      (`KismetSystemLibrary.PrintString` (`KismetStringLibrary.Concat_StrStr` (`KismetStringLibrary.Conv_IntToString` _output_get_2) " / " (`KismetStringLibrary.Conv_IntToString` (`self.WallGenerateNumOneGame`)) " Generate Wall Success") true false (struct :`G` 1.0 :`A` 1.0) 3.0))
    (:`OnFail`
      (`KismetSystemLibrary.PrintString` "Failed..."))))

(fn `DeleteWall`
  (params (NewParam :type "/Game/BluePrint/BP_Wall2PMask Object Reference"))
  (`self.K2_DestroyActor` NewParam)
  (bind _output_get (set `self.DeleteWallNum` (+ (`self.DeleteWallNum`) 1)))
  (`KismetSystemLibrary.PrintString` (`KismetStringLibrary.Concat_StrStr` (`KismetStringLibrary.Conv_IntToString` _output_get) " / " (`KismetStringLibrary.Conv_IntToString` (`self.WallGenerateNumOneGame`)) " Delete Wall") true true (struct :`G` 1.0 :`A` 1.0) 3.0)
  (if (>= (`self.DeleteWallNum`) (`self.WallGenerateNumOneGame`))
    (`KismetSystemLibrary.PrintString` "Game Clear !" true true (struct :`G` 1.0 :`A` 1.0) 10.0)
    (set `self.GameState` "NewEnumerator1")))

(fn `GenerateWall`
  (locals (GeneratedStaticMeshActor :type "StaticMeshActor Object Reference"))
  (bind _returnvalue (`|SpawnActorFromClass` "/Game/BluePrint/BP_Wall2PMask.BP_Wall2PMask_C" (`KismetMathLibrary.MakeTransform` (`self.WallGeneratePos`) (struct :`Yaw` 180.0) (`self.WallScale`)) "Undefined" "OverrideRootScale" null null))
  ;[1 1 1] 初期値設定
  (set `/Game/BluePrint/BP_Wall2PMask.WallStartPos` (`self.WallGeneratePos`) _returnvalue)
  (set `/Game/BluePrint/BP_Wall2PMask.WallGoalPos` (`self.WallDeletePos`) _returnvalue)
  (set `/Game/BluePrint/BP_Wall2PMask.WallLifeTime` (`self.WallLifeTimeStartToGoal`) _returnvalue))

(fn `UserConstructionScript`)