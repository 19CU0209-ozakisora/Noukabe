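; WallAction captures a render target as a mask image when V is pressed while freezing the BP_EasyHuman found at BeginPlay.
; It exports NewTextureRenderTarget2D as a PNG to a hard-coded SceneCapture folder and sets the human mesh's play rate to zero.
; The export callback waits, then resumes playback and clears the re-entry flag.
; A timeline animating the cut-out wall (WallMinus) falling over is present but never runs.
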(event `self.ReceiveBeginPlay`
  (bind _returnvalue (`GameplayStatics.GetActorOfClass` "/Game/BluePrint/BP_Easyhuman.BP_EasyHuman_C"))
  (bind _output_get (set `self.Human` _returnvalue))
  (if (`KismetSystemLibrary.IsValid` _output_get)
    (`KismetSystemLibrary.PrintString` "Hello")))

(event `self.ReceiveActorBeginOverlap`
  (params (OtherActor :type "Actor Object Reference")))

(event `Key|V`
  (params (Key :type "Key Structure"))
  (:`Pressed`
    (if (not (`self.NewVar_0`))
      (set `self.NewVar_0` true)
      (`KismetSystemLibrary.PrintString` "Caputure" true true (struct :`G` 0.66 :`B` 1.0 :`A` 1.0) 5.0)
      (`ImageWriteBlueprintLibrary.ExportToDisk` "/Game/Other/NewTextureRenderTarget2D.NewTextureRenderTarget2D" "C:\\Users\\yuto1\\Documents\\Noukabe\\Noukabe\\Content\\texture\\SceneCapture\\MaskTex" (make `ImageWriteOptions` "PNG" (delegate `カスタムイベント_0`)))
      (`SkeletalMeshComponent.SetPlayRate` (`/Game/BluePrint/BP_Easyhuman.HumanSkeletalMesh` (`self.Human`)) 0.0))))

(event `カスタムイベント_0`
  (params (bSuccess :type Boolean))
  (`KismetSystemLibrary.Delay` 3.0)
  (`SkeletalMeshComponent.SetPlayRate` (`/Game/BluePrint/BP_Easyhuman.HumanSkeletalMesh` (`self.Human`)) 1.0)
  (set `self.NewVar_0` false))

(fn `UserConstructionScript`)