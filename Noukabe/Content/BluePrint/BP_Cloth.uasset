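; BP_Cloth is a cloth actor that slides sideways to open or close, apparently as one half of a two-sided pair such as curtains.
; Each open or close call nudges the actor one fixed step along local Y, so continuous motion depends on repeated calls.
; The Side flag mirrors direction and negates the limits, which are checked against ClothPrototype's world X before each step.
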(event `open`
  (bind _returnvalue_x (`KismetMathLibrary.BreakVector` (`SceneComponent.K2_GetComponentLocation` (`self.cloth_prototype`))))
  ;[1 1 1] 開く
  (`|ExecutionSequence`
    (:`then_0`
      (set `self.pos` _returnvalue_x))
    (:`then_1`
      (if (`self.Side`)
        (if (> (`self.toMoveOpen`) (`self.pos`))
          (`self.K2_AddActorLocalOffset` (0.0 4.0 0.0)))
        (elif (> (`self.pos`) (* (`self.toMoveOpen_0`) -1.0))
          (`self.K2_AddActorLocalOffset` (0.0 -4.0 0.0)))))))

(event `close`
  (bind _returnvalue_x (`KismetMathLibrary.BreakVector` (`SceneComponent.K2_GetComponentLocation` (`self.cloth_prototype`))))
  ;[1 1 1] 閉じる
  (`|ExecutionSequence`
    (:`then_0`
      (set `self.pos2` _returnvalue_x))
    (:`then_1`
      (if (`self.Side`)
        (if (<= (`self.toMoveClose`) (`self.pos2`))
          (`self.K2_AddActorLocalOffset` (0.0 -4.0 0.0)))
        (elif (<= (`self.pos2`) (* (`self.toMoveClose_0`) -1.0))
          (`self.K2_AddActorLocalOffset` (0.0 4.0 0.0)))))))

(fn `UserConstructionScript`)