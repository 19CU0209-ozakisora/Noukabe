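; In-game manager that runs a wall-flow round through Preparation, Game and Clear states, driven from Tick.
; BeginPlay caches start and end positions from marker actors and gathers wall meshes by scanning a content folder through the Asset Registry.
; After a start delay, it spawns randomly meshed walls at intervals up to a set count.
; DeleteWall counts removals to trigger Clear, which plays Niagara effects once and opens the Result level.
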(event `self.ReceiveBeginPlay`
  ;[1 1 1] 壁生成位置設定
  (bind _output_get (set `self.WallGeneratePos` (`SceneComponent.K2_GetComponentLocation` (`self.WallGeneratePosActor`))))
  (`KismetSystemLibrary.PrintString` (`KismetStringLibrary.Concat_StrStr` "Wall Generate Pos : " (`KismetStringLibrary.Conv_VectorToString` _output_get)) true true (struct :`G` 1.0 :`A` 1.0) 5.0)
  ;[1 1 1] 壁削除位置設定
  (bind _output_get_2 (set `self.WallDeletePos` (`SceneComponent.K2_GetComponentLocation` (`self.WallDeletePosActor`))))
  (`KismetSystemLibrary.PrintString` (`KismetStringLibrary.Concat_StrStr` "Wall Delete Pos : " (`KismetStringLibrary.Conv_VectorToString` _output_get_2)) true true (struct :`G` 1.0 :`A` 1.0) 5.0)
  ;[1 1 1] 壁を流す長さ算出（現時点で算出結果は未使用）
  (bind _output_get_3 (set `self.WallFlowDistance` (`KismetMathLibrary.VSizeXY` (- (`self.WallGeneratePos`) (`self.WallDeletePos`)))))
  (`KismetSystemLibrary.PrintString` (`KismetStringLibrary.Concat_StrStr` "WallFlowDistance : " (`KismetStringLibrary.Conv_DoubleToString` _output_get_3)) true true (struct :`G` 1.0 :`A` 1.0) 5.0)
  ;[1 1 1] ゲーム状態設定
  (set `self.GameState` "NewEnumerator4")
  (bind (_outassetdata _returnvalue) (`AssetRegistry.GetAssetsByPath` (`AssetRegistryHelpers.GetAssetRegistry`) "/Game/Mesh/Wall" false false))
  (if _returnvalue
    (for _array_element _outassetdata
      (if (== (`AssetRegistryHelpers.GetClass` _array_element) "/Script/Engine.StaticMesh")
        (bind _asstatic_mesh (cast `StaticMesh` (`AssetRegistryHelpers.GetAsset` _array_element)))
        (`KismetArrayLibrary.Array_Add` (`self.WallsMesh`) _asstatic_mesh)))
    (`KismetSystemLibrary.PrintString` (`KismetStringLibrary.Concat_StrStr` "Wall Kind : " (`KismetStringLibrary.Conv_IntToString` (`KismetArrayLibrary.Array_Length` (`self.WallsMesh`)))) true true (struct :`G` 0.66 :`B` 1.0 :`A` 1.0) 5.0)))

(event `self.ReceiveTick`
  (params (DeltaSeconds :type "Float (single-precision)"))
  (set `self.DeltaTime` DeltaSeconds)
  (`|ExecutionSequence`
    (:`then_0`
      (switch `/Game/Other/InGameState` (`self.GameState`)
        (:`NewEnumerator4`
          (`KismetSystemLibrary.Delay` (`self.StartWallFlowTime`))
          (set `self.GameState` "NewEnumerator0")
          (`KismetSystemLibrary.PrintString` "GameStart!" true true (struct :`G` 1.0 :`A` 1.0) 3.0))
        (:`NewEnumerator0`
          (if (< (`self.GeneratedWallNum`) (`self.WallGenerateNumOneGame`))
            (bind _output_get (set `self.WallGenerateTimeCnt` (+ (`self.DeltaTime`) (`self.WallGenerateTimeCnt`))))
            (if (>= _output_get (`self.WallGenerateSpan`))
              (set `self.WallGenerateTimeCnt` 0.0)
              (`self.GenerateWall`)
              (bind _output_get_2 (set `self.GeneratedWallNum` (+ (`self.GeneratedWallNum`) 1)))
              (`KismetSystemLibrary.PrintString` (`KismetStringLibrary.Concat_StrStr` (`KismetStringLibrary.Conv_IntToString` _output_get_2) " / " (`KismetStringLibrary.Conv_IntToString` (`self.WallGenerateNumOneGame`)) " Generate Wall Success") true false (struct :`G` 1.0 :`A` 1.0) 3.0))))
        (:`NewEnumerator1`
          (`/Engine/EditorBlueprintResources/StandardMacros.DoOnce` false
            (:`Completed`
              (`KismetSystemLibrary.Delay` 2.0)
              (`AddComponent|NODE_AddNiagaraComponent-0` :`RelativeTransform` (`SceneComponent.GetRelativeTransform` (`self.GameClearEffectGenePos01`)))
              (`AddComponent|NODE_AddNiagaraComponent-1` :`RelativeTransform` (`SceneComponent.GetRelativeTransform` (`self.GameClearEffectGenePos02`)))
              (`KismetSystemLibrary.Delay` 8.0)
              (`GameplayStatics.OpenLevel` "Result"))))))
    (:`then_1`
      (`KismetSystemLibrary.PrintString` (`KismetStringLibrary.Concat_StrStr` "GameState : " (`|GetEnumeratorNameAsString` (`self.GameState`))) true true (struct :`G` 1.0 :`A` 1.0) (`self.DeltaTime`)))))

(fn `DeleteWall`
  (params (NewParam :type "/Game/BluePrint/BP_Wall Object Reference"))
  (`self.K2_DestroyActor` NewParam)
  (bind _output_get (set `self.DeleteWallNum` (+ (`self.DeleteWallNum`) 1)))
  (`KismetSystemLibrary.PrintString` (`KismetStringLibrary.Concat_StrStr` (`KismetStringLibrary.Conv_IntToString` _output_get) " / " (`KismetStringLibrary.Conv_IntToString` (`self.WallGenerateNumOneGame`)) " Delete Wall") true true (struct :`G` 1.0 :`A` 1.0) 3.0)
  (if (>= (`self.DeleteWallNum`) (`self.WallGenerateNumOneGame`))
    (`KismetSystemLibrary.PrintString` "Game Clear !" true true (struct :`G` 1.0 :`A` 1.0) 10.0)
    (set `self.GameState` "NewEnumerator1")))

(fn `GenerateWall`
  (locals (GeneratedStaticMeshActor :type "StaticMeshActor Object Reference"))
  (bind _wallsmesh (`self.WallsMesh`))
  (bind _returnvalue (`|SpawnActorFromClass` "/Game/BluePrint/BP_Wall.BP_Wall_C" (`KismetMathLibrary.MakeTransform` (`self.WallGeneratePos`) (struct :`Yaw` 180.0) (`self.WallScale`)) "Undefined" "OverrideRootScale" null null))
  ;[1 1 1] 初期値設定
  (set `/Game/BluePrint/BP_Wall.WallStartPos` (`self.WallGeneratePos`) _returnvalue)
  (set `/Game/BluePrint/BP_Wall.WallGoalPos` (`self.WallDeletePos`) _returnvalue)
  (set `/Game/BluePrint/BP_Wall.WallLifeTime` (`self.WallLifeTimeStartToGoal`) _returnvalue)
  ;[1 1 1] 壁のメッシュをランダムで設定
  (`StaticMeshComponent.SetStaticMesh` (`/Game/BluePrint/BP_Wall.WallMesh` _returnvalue) (`|GetArrayItem` _wallsmesh (`KismetMathLibrary.RandomInteger` (`KismetArrayLibrary.Array_Length` _wallsmesh)))))

(fn `UserConstructionScript`)