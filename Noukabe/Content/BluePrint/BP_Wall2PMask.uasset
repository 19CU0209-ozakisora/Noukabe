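; BP_Wall2PMask is a battle-mode wall actor that travels from a start position to a goal position over its lifetime.
; After a start delay it enables Tick, which accumulates elapsed time into a progress ratio and linearly interpolates the actor's location.
; Once progress passes the end, it prints a debug message and asks BP_InGameManager_BattleMode to delete it instead of destroying itself.
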(event `self.ReceiveBeginPlay`
  (`KismetSystemLibrary.Delay` (`self.MoveDelay`))
  (`self.SetActorTickEnabled` true))

(event `self.ReceiveTick`
  (params (DeltaSeconds :type "Float (single-precision)"))
  (bind _wallprogress (`self.WallProgress`))
  (set `self.WallTimeSinceGenerate` (+ DeltaSeconds (`self.WallTimeSinceGenerate`)))
  (if (!= (`self.WallTimeSinceGenerate`) 0.0)
    (set `self.WallProgress` (/ (`self.WallTimeSinceGenerate`) (`self.WallLifeTime`)))
    (else
      (set `self.WallProgress` 0.0)))
  (if (> _wallprogress 1.0)
    (`KismetSystemLibrary.PrintString` "Wall is Goal" true false (struct :`G` 1.0 :`A` 1.0) 3.0)
    ;[1 1 1] 終点についてたら削除処理をお願いする
    (bind _returnvalue (`GameplayStatics.GetActorOfClass` "/Game/BluePrint/BP_InGameManager_BattleMode.BP_InGameManager_BattleMode_C"))
    (`/Game/BluePrint/BP_InGameManager_BattleMode.DeleteWall` _returnvalue self)
    (else
      ;[1 1 1] 壁を移動させる
      (`self.K2_SetActorLocation` (`|EaseFunction` "Linear" _wallprogress (`self.WallStartPos`) (`self.WallGoalPos`))))))

(fn `UserConstructionScript`)