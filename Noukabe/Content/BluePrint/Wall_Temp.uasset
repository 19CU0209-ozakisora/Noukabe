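; Wall_Temp is a moving wall actor that slides its Cube a fixed step along world -Y every tick, without sweep or delta-time scaling.
; It records its spawn location on BeginPlay and destroys itself once the Cube strays beyond DestroyMovement from it on any axis.
; Cube overlap and hit events share one debug print naming the other actor.
; CollisionChange is an empty stub.
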(event `self.ReceiveBeginPlay`
  (set `self.CreateLocation` (`self.K2_GetActorLocation`)))

(event `self.ReceiveTick`
  (params (DeltaSeconds :type "Float (single-precision)"))
  (bind (_createlocation_x _createlocation_y _createlocation_z) (`KismetMathLibrary.BreakVector` (`self.CreateLocation`)))
  (bind (_returnvalue_x _returnvalue_y _returnvalue_z) (`KismetMathLibrary.BreakVector` (`SceneComponent.K2_GetComponentLocation` (`self.Cube`))))
  (`SceneComponent.K2_AddWorldOffset` (`self.Cube`) (0.0 -1.0 0.0) false false)
  (if (or (> (`KismetMathLibrary.Abs` (- _returnvalue_x _createlocation_x)) (`self.DestroyMovement`)) (> (`KismetMathLibrary.Abs` (- _returnvalue_y _createlocation_y)) (`self.DestroyMovement`)) (> (`KismetMathLibrary.Abs` (- _returnvalue_z _createlocation_z)) (`self.DestroyMovement`)))
    (`self.K2_DestroyActor`)))

(event `self.Cube.OnComponentBeginOverlap`
  (params (OverlappedComponent :type "PrimitiveComponent Object Reference") (OtherActor :type "Actor Object Reference") (OtherComp :type "PrimitiveComponent Object Reference") (OtherBodyIndex :type Integer) (bFromSweep :type Boolean) (SweepResult :type "HitResult Structure (by ref)"))
  (`KismetSystemLibrary.PrintString` (`KismetStringLibrary.Concat_StrStr` "壁が" (`KismetSystemLibrary.GetObjectName` (stale `self.Cube.OnComponentHit` OtherActor)) "に衝突") true true (struct :`G` 0.66 :`B` 1.0 :`A` 1.0) 1.0 :!label _label))

(event `self.Cube.OnComponentHit`
  (params (HitComponent :type "PrimitiveComponent Object Reference") (OtherActor :type "Actor Object Reference") (OtherComp :type "PrimitiveComponent Object Reference") (NormalImpulse :type "Vector Structure") (Hit :type "HitResult Structure (by ref)"))
  (goto _label))

(fn `CollisionChange`)

(fn `UserConstructionScript`)