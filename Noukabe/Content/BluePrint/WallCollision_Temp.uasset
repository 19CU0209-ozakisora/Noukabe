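; WallCollision_Temp is a temporary collision test actor that detects when a tagged tracker component enters or leaves its Sphere.
; Sphere begin and end overlap events check the other component for a tag built from the TargetTracker enum's name.
; On a match, each event prints a "Start Overlap" or "End Overlap" debug string followed by that tracker name; no other gameplay logic is wired.
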(event `self.Sphere.OnComponentBeginOverlap`
  (params (OverlappedComponent :type "PrimitiveComponent Object Reference") (OtherActor :type "Actor Object Reference") (OtherComp :type "PrimitiveComponent Object Reference") (OtherBodyIndex :type Integer) (bFromSweep :type Boolean) (SweepResult :type "HitResult Structure (by ref)"))
  (bind _returnvalue (`KismetStringLibrary.Conv_StringToName` (`|GetEnumeratorNameAsString` (`self.TargetTracker`))))
  (if (`ActorComponent.ComponentHasTag` OtherComp _returnvalue)
    (`KismetSystemLibrary.PrintString` (`KismetStringLibrary.Concat_StrStr` "Start Overlap" (`KismetStringLibrary.Conv_NameToString` _returnvalue)))))

(event `self.Sphere.OnComponentEndOverlap`
  (params (OverlappedComponent :type "PrimitiveComponent Object Reference") (OtherActor :type "Actor Object Reference") (OtherComp :type "PrimitiveComponent Object Reference") (OtherBodyIndex :type Integer))
  (bind _returnvalue (`KismetStringLibrary.Conv_StringToName` (`|GetEnumeratorNameAsString` (`self.TargetTracker`))))
  (if (`ActorComponent.ComponentHasTag` OtherComp _returnvalue)
    (`KismetSystemLibrary.PrintString` (`KismetStringLibrary.Concat_StrStr` "End Overlap" (`KismetStringLibrary.Conv_NameToString` _returnvalue)))))

(fn `UserConstructionScript`)